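; Player character Blueprint handling camera-relative movement, look, jump, sprint, roll and combo attacks through Enhanced Input.
; IA_Mobility sprints on hold, draining StaminaComponent on Tick with pause and resume around exhaustion, and rolls on tap.
; Roll montages play forward, or by input direction when orient-to-movement is off (lock-on), with movement input stopped until completion.
; Attacks step through a combo type array, advancing only when CombatComponent accepts the attack.
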(event Custom|StopSprint
  ;[0.15 0.15 0.15 0.5] 이동
  ;;[0.15 0.15 0.15 0.5] 이동 보조:달리기, 구르기
  ;;;[0.15 0.15 0.15 0.5] 달리기 해제: 기본 속도로 변경
  (Variables|/Script/Engine.CharacterMovementComponent|SetMaxWalkSpeed (Variables|Character|GetCharacterMovement) (Variables|이동|GetDefaultGroundSpeed))
  ;;;[0.15 0.15 0.15 0.5] 스태미나 회복 시작
  (Default|StartRechargeDelay (Variables|Default|GetStamina%20Component)))

(event Custom|StartSprint
  ;[0.15 0.15 0.15 0.5] 이동
  ;;[0.15 0.15 0.15 0.5] 이동 보조:달리기, 구르기
  ;;;[0.15 0.15 0.15 0.5] 달리기 시작: 달리기 속도로 변경
  (Variables|/Script/Engine.CharacterMovementComponent|SetMaxWalkSpeed (Variables|Character|GetCharacterMovement) (Variables|Movement|GetSprintSpeed))
  ;;;[0.15 0.15 0.15 0.5] 스태미나 회복 중단
  (Default|StopRecharge (Variables|Default|GetStamina%20Component)))

(event Custom|StartAttack
  ;[0.15 0.15 0.15 0.5] 일반 공격: 4단 콤보
  ;;[0.15 0.15 0.15 0.5] 콤보 중간에도 캐릭터 회전이 가능하도록 Input Movement 활성/비활성도 수행
  (CallFunction|StopInputMovement)
  (Default|StartAttack (Variables|Default|GetCombatComponent)))

(event Custom|EndAttack
  ;[0.15 0.15 0.15 0.5] 일반 공격: 4단 콤보
  ;;[0.15 0.15 0.15 0.5] 콤보 중간에도 캐릭터 회전이 가능하도록 Input Movement 활성/비활성도 수행
  (Default|EndAttack (Variables|Default|GetCombatComponent))
  (CallFunction|RestartInputMovement))

(event Custom|ResetCombo
  ;[0.15 0.15 0.15 0.5] 일반 공격: 4단 콤보
  ;;[0.15 0.15 0.15 0.5] 콤보 횟수 초기화
  (Variables|Default|SetComboIndex 0))

(event Input|EnhancedActionEvents|EnhancedInputActionIA_Move
  (params (ActionValue :type Vector%202D%20Structure) (ElapsedSeconds :type Float%20%28double-precision%29) (TriggeredSeconds :type Float%20%28double-precision%29) (InputAction :type Input%20Action%20Object%20Reference :default "/Game/MyContents/Input/Actions/IA_Move.IA_Move"))
  ;[0.15 0.15 0.15 0.5] 이동
  ;;[0.15 0.15 0.15 0.5] 입력: 이동 (WASD, 방향키)
  (:Triggered
    (bind _output_get (Variables|이동|SetCurrentMoveInput ActionValue))
    (|LeftRightMove (.X (Math|Vector2D|BreakVector2D _output_get)))
    (|ForwardBackward (.Y (Math|Vector2D|BreakVector2D _output_get))))
  (:Completed
    (Variables|이동|SetCurrentMoveInput "")))

(event Input|EnhancedActionEvents|EnhancedInputActionIA_Jump
  (params (ActionValue :type Boolean) (ElapsedSeconds :type Float%20%28double-precision%29) (TriggeredSeconds :type Float%20%28double-precision%29) (InputAction :type Input%20Action%20Object%20Reference :default "/Game/MyContents/Input/Actions/IA_Jump.IA_Jump"))
  ;[0.15 0.15 0.15 0.5] 이동
  ;;[0.15 0.15 0.15 0.5] 입력: 점프 (Space Bar)
  (:Started
    (if (Variables|Default|GetbCanJump)
      (switch Utilities|FlowControl|Switch|SwitchonEMovementMode (Variables|/Script/Engine.CharacterMovementComponent|GetMovementMode (Variables|Character|GetCharacterMovement))
        (:MOVE_Walking
          (Character|Jump)))))
  (:Completed
    (Character|StopJumping)))

(event Input|EnhancedActionEvents|EnhancedInputActionIA_Mobility
  (params (ActionValue :type Boolean) (ElapsedSeconds :type Float%20%28double-precision%29) (TriggeredSeconds :type Float%20%28double-precision%29) (InputAction :type Input%20Action%20Object%20Reference :default "/Game/MyContents/Input/Actions/IA_Mobility.IA_Mobility"))
  (bind _rollanimmontage (Variables|Default|GetRollAnimMontage))
  (bind _currentmoveinput (Variables|이동|GetCurrentMoveInput))
  (bind _rollanimmontage_2 (Variables|Default|GetRollAnimMontage))
  (bind (_value _returnvalue) (Utilities|Map|Find _rollanimmontage _currentmoveinput))
  (bind (_value_2 _returnvalue_2) (Utilities|Map|Find :TargetMap _rollanimmontage_2))
  ;[0.15 0.15 0.15 0.5] 이동
  ;;[0.15 0.15 0.15 0.5] 이동 보조:달리기, 구르기
  (:Triggered
    ;;;[0.15 0.15 0.15 0.5] 달리기 실행: 달리기 속도로 변경
    (if (and (not (Variables|Movement|GetbIsSprinting)) (> ElapsedSeconds (Variables|Default|GetHoldTimeThreshold)))
      (CallFunction|StartSprint)
      (Variables|Movement|SetbIsSprinting true)))
  (:Completed
    (if (Variables|Movement|GetbIsSprinting)
      (CallFunction|StopSprint)
      (Variables|Movement|SetbIsSprinting false)
      (Variables|이동|SetbIsStaminaExhausted false)
      (elif (Variables|/Script/Engine.CharacterMovementComponent|GetbOrientRotationToMovement (Variables|Character|GetCharacterMovement))
        ;;;[0.15 0.15 0.15 0.5] 락온 아닐 때: 캐릭터가 항상 입력 방향을 바라보고 있음
        ;;; ->  앞으로 구르기
        (if _returnvalue_2
          (Utilities|PlayMontagee _value_2)
          (else
            (Development|PrintString "Error: No Default Roll Animation Montage" true true "(R=1.000000,G=0.000000,B=0.000000,A=1.000000)" 5.0)))
        (else
          ;;;[0.15 0.15 0.15 0.5] 락온 상태: 캐릭터 기준으로 방향 정해서 구르기
          ;;;;[0.15 0.15 0.15 0.5] 입력 방향 알아내기
          (if _returnvalue
            (Utilities|PlayMontagee _value)
            (else
              (Development|PrintString (Class|KismetStringLibrary|BuildStringVector2d "" "Error: Invalid Input Direciton " _currentmoveinput) true true "(R=1.000000,G=0.000000,B=0.000000,A=1.000000)" 5.0))))))))

(event Input|EnhancedActionEvents|EnhancedInputActionIA_MouseLook
  (params (ActionValue :type Vector%202D%20Structure) (ElapsedSeconds :type Float%20%28double-precision%29) (TriggeredSeconds :type Float%20%28double-precision%29) (InputAction :type Input%20Action%20Object%20Reference :default "/Game/MyContents/Input/Actions/IA_MouseLook.IA_MouseLook"))
  (bind (_x _y) (Math|Vector2D|BreakVector2D ActionValue))
  ;[0.15 0.15 0.15 0.5] 입력: 카메라 회전 (마우스 이동)
  (Pawn|Input|AddControllerYawInput _x)
  (Pawn|Input|AddControllerPitchInput _y))

(event Input|EnhancedActionEvents|EnhancedInputActionIA_Attack
  (params (ActionValue :type Boolean) (ElapsedSeconds :type Float%20%28double-precision%29) (TriggeredSeconds :type Float%20%28double-precision%29) (InputAction :type Input%20Action%20Object%20Reference :default "/Game/MyContents/Input/Actions/IA_Attack.IA_Attack"))
  (bind _comboattacktype (Variables|Attack|GetComboAttackType))
  (bind _attacktype (Variables|Attack|GetAttackType))
  (bind _comboindex (Variables|Default|GetComboIndex))
  (bind _output (Utilities|Array|Get(acopy) _comboattacktype _comboindex))
  (bind (_value _returnvalue) (Utilities|Map|Find _attacktype _output))
  ;[0.15 0.15 0.15 0.5] 일반 공격: 4단 콤보
  (:Started
    (if _returnvalue
      (bind _bsuccess (Default|Attack (Variables|Default|GetCombatComponent) _value))
      ;;[0.15 0.15 0.15 0.5] Combo Index 증가: 공격 실행 후 다음 콤보 준비
      (if _bsuccess
        (if (< (Variables|Default|GetComboIndex) (- (Utilities|Array|Length (Variables|Attack|GetComboAttackType)) 1))
          (Math|Integer|IncrementInt (Variables|Default|GetComboIndex))
          (else
            (CallFunction|ResetCombo))))
      (else
        (Development|PrintString (Utilities|String|BuildString(Name) "" "Error: Invalidate Attack type for " (Utilities|Name|EnumtoName _output) "") true true "(R=1.000000,G=0.000000,B=0.000000,A=1.000000)" 5.0)))))

(event EventBeginPlay
  (Variables|/Script/Engine.CharacterMovementComponent|SetMaxWalkSpeed (Variables|Character|GetCharacterMovement) (Variables|이동|GetDefaultGroundSpeed))
  (Default|Initialize (Variables|Default|GetCombatComponent) self (Variables|Default|GetStamina%20Component))
  (Default|EquipWeapon (Variables|Default|GetCombatComponent) (Variables|Default|GetDefaultWeaponClass))
  (EventDispatchers|BindEventtoOnAttackEnded (Variables|Default|GetCombatComponent) (EventDispatchers|CreateEvent :!event Custom|ResetCombo)))

(event Collision|EventActorBeginOverlap
  (params (OtherActor :type Actor%20Object%20Reference)))

(event EventTick
  (params (DeltaSeconds :type Float%20%28single-precision%29))
  ;[0.15 0.15 0.15 0.5] 달리기 중 스태미나 소비
  (if (Variables|이동|GetbIsStaminaExhausted)
    (if (not (< (Variables|/Game/MyContents/Components/BPC_Stamina.BPC_Stamina_C|GetCurrentStamina (Variables|Default|GetStamina%20Component)) (Variables|이동|GetSprintRecoveryThreshold)))
      (Variables|이동|SetbIsStaminaExhausted false)
      (CallFunction|StartSprint))
    (elif (and (Variables|Movement|GetbIsSprinting) (> (Class|KismetMathLibrary|VSizeXYSquared (Transformation|GetVelocity)) 0.0))
      (bind _bsuccess (Default|TryConsumeStaminaContinuous (Variables|Default|GetStamina%20Component) (* DeltaSeconds (Variables|이동|GetSprintStaminaCostPerSecond))))
      (if (not _bsuccess)
        (Variables|이동|SetbIsStaminaExhausted true)
        (CallFunction|StopSprint)))))

(event Game|Damage|EventAnyDamage
  (params (Damage :type Float%20%28single-precision%29) (DamageType :type Damage%20Type%20Object%20Reference) (InstigatedBy :type Controller%20Object%20Reference) (DamageCauser :type Actor%20Object%20Reference))
  ;[0.15 0.15 0.15 0.5] 일반 공격: 4단 콤보
  ;;[0.15 0.15 0.15 0.5] 피격
  (|CallParentFunction Damage DamageType InstigatedBy DamageCauser))

(fn ConstructionScript)