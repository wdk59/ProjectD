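; Elite skeleton enemy Blueprint that adds a cooldown-gated Roar skill with an area attack to its parent's behavior.
; OnSkillRoar checks availability and CombatComponent.TryAttack, then RoarAttack disables movement and plays the attack montage.
; Montage completion restores walking and starts a cooldown timer, which re-enables the skill unless the skeleton is dead.
; A separate PerformSkillRoar event applies the area attack through CombatComponent.
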(event Custom|RoarAttack
  (params (InAttackData :type ST%20Attack%20Data%20Structure))
  ;[0.15 0.15 0.15 0.5] 스킬: 포효
  (Variables|Default|SetbCanUseSkillRoar false)
  (Pawn|Components|CharacterMovement|DisableMovement (Variables|Character|GetCharacterMovement))
  (Animation|Montage|PlayMontage (Variables|Character|GetMesh) (.AttackMontage (Utilities|Struct|BreakST_AttackData InAttackData))
    (:OnCompleted
      (Pawn|Components|CharacterMovement|SetMovementMode (Variables|Character|GetCharacterMovement) "MOVE_Walking" 0)
      (CallFunction|StartRoarCooldown))))

(event Custom|StartRoarCooldown
  ;[0.15 0.15 0.15 0.5] 스킬: 포효
  ;;[0.15 0.15 0.15 0.5] 포효 후 쿨다운 제어
  (Utilities|Time|SetTimerbyEvent (delegate Custom|OnRoarCooldownCompleted) (Variables|Combat|GetRoarCooldown)))

(event Custom|OnRoarCooldownCompleted
  ;[0.15 0.15 0.15 0.5] 스킬: 포효
  ;;[0.15 0.15 0.15 0.5] 포효 후 쿨다운 제어
  (if (not (Variables|/Game/MyContents/Components/BPC_Health.BPC_Health_C|GetbIsDead (Variables|Default|GetHealthComponent)))
    (Variables|Default|SetbCanUseSkillRoar true)))

(event EventBeginPlay
  (|CallParentFunction)
  (Variables|Default|SetbCanUseSkillRoar true))

(event Collision|EventActorBeginOverlap
  (params (OtherActor :type Actor%20Object%20Reference))
  (|CallParentFunction OtherActor) ; 지금 이 노드는 비활성 상태입니다. \n핀을 끌어서 다른 노드를 연결하면 활성화됩니다.
)

(event EventTick
  (params (DeltaSeconds :type Float%20%28single-precision%29))
  (|CallParentFunction DeltaSeconds))

(event EventPerformSkillRoar
  ;[0.15 0.15 0.15 0.5] 스킬: 포효
  (Default|PerformAreaAttack (Variables|Default|GetCombatComponent) (Variables|Combat|GetRoarAreaAttackData)))

(fn ConstructionScript
  (|CallParentFunction))

(fn OnSkillRoar
  (bind _roarattackdata (Variables|Combat|GetRoarAttackData))
  (bind _bcanuseskillroar (Variables|Default|GetbCanUseSkillRoar))
  (if _bcanuseskillroar
    (bind _bsuccess (Default|TryAttack (Variables|Default|GetCombatComponent) _roarattackdata))
    (if _bsuccess
      (CallFunction|RoarAttack _roarattackdata)
      (return (and _bsuccess _bcanuseskillroar)))))