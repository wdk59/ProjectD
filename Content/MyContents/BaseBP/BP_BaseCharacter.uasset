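; BP_BaseCharacter is a base character Blueprint providing shared attack, damage and team behavior.
; PlayAttack plays the given montage on the Mesh while move input and jumping are blocked, restoring both only on the montage's Completed output.
; AnyDamage forwards damage to HealthComponent and prints the damage causer and current health for debugging.
; GetTeam exposes the character's Team value.
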(event Custom|StopInputMovement
  ;[0.15 0.15 0.15 0.5] 이동 입력 제어
  (Input|SetIgnoreMoveInput (Pawn|GetController) true)
  (Variables|Default|SetbCanJump false))

(event Custom|RestartInputMovement
  ;[0.15 0.15 0.15 0.5] 이동 입력 제어
  (Input|ResetIgnoreMoveInput (Pawn|GetController))
  (Variables|Default|SetbCanJump true))

(event Custom|PlayAttackMontage
  (params (InAnimMontage :type Anim%20Montage%20Object%20Reference))
  (CallFunction|StopInputMovement)
  (Animation|Montage|PlayMontage (Variables|Character|GetMesh) InAnimMontage
    (:OnCompleted
      (CallFunction|RestartInputMovement))))

(event EventBeginPlay)

(event Collision|EventActorBeginOverlap
  (params (OtherActor :type Actor%20Object%20Reference)))

(event EventTick
  (params (DeltaSeconds :type Float%20%28single-precision%29)))

(event Game|Damage|EventAnyDamage
  (params (Damage :type Float%20%28single-precision%29) (DamageType :type Damage%20Type%20Object%20Reference) (InstigatedBy :type Controller%20Object%20Reference) (DamageCauser :type Actor%20Object%20Reference))
  (bind _healthcomponent (Variables|Default|GetHealthComponent))
  (Default|ReceiveDamage _healthcomponent Damage)
  ;[1 0 0 0.5] Debug: 피격 및 체력 확인
  (Development|PrintString (Utilities|String|BuildString(Object) "" "Get Damage by " DamageCauser) true true "(R=0.000000,G=1.000000,B=0.000000,A=1.000000)")
  (bind _outhealth (Default|GetHealth _healthcomponent))
  (Development|PrintString (Class|KismetStringLibrary|BuildStringDouble "" "Now Health: " _outhealth) true true "(R=0.000000,G=1.000000,B=0.000000,A=1.000000)"))

(fn ConstructionScript)

(fn PlayAttack
  (params (InAttackMontage :type Anim%20Montage%20Object%20Reference))
  (CallFunction|PlayAttackMontage InAttackMontage))

(fn GetTeam
  (return (Variables|Default|GetTeam)))