(event EventBeginPlay)

(event EventTick
  (params (DeltaSeconds :type Float%20%28single-precision%29)))

(fn OnWeaponHit
  (params (InHitActor :type Actor%20Object%20Reference))
  (Game|Damage|ApplyDamage InHitActor (.damage (Variables|Default|GetCurrentAttackData)) 0 0)
  ;[0.15 0.15 0.15 0.5] Debug: Weapon Hit Actor
  (Development|PrintString (Utilities|String|BuildString(Object) "" "Hit Actor: " InHitActor) true true "(R=0.000000,G=1.000000,B=0.000000,A=1.000000)"))

(fn EquipWeapon
  (params (InWeapon :type BP%20Sword%20Class%20Reference))
  (bind _returnvalue (Game|SpawnActorfromClass InWeapon (Transformation|GetActorTransform (Variables|Default|GetOwnerCharacter)) "Undefined" "MultiplyWithRoot" 0 0))
  (Transformation|AttachComponentToComponent _returnvalue (Variables|/Script/Engine.Character|GetMesh (Variables|Default|GetOwnerCharacter)) "SwordSocket" "SnapToTarget" "SnapToTarget" "SnapToTarget" true)
  (bind _output_get (Variables|Default|SetCurrentWeapon _returnvalue))
  (Default|Initialize (Variables|/Game/MyContents/Weapons/BP_Sword.BP_Sword_C|GetWeaponComponent _output_get) (Variables|Default|GetOwnerCharacter) (Variables|/Game/MyContents/Weapons/BP_Sword.BP_Sword_C|GetMesh _output_get)))

(fn TryAttack
  (params (InAttackData :type ST%20Attack%20Data%20Structure))
  (bind (_attackmontage _damage _staminacost) (Utilities|Struct|BreakST_AttackData InAttackData))
  (bind _ownerstaminacomponentt (Variables|Default|GetOwnerStaminaComponentt))
  (if (Variables|Default|GetbIsAttacking)
    (return false)
    (else
      (Utilities|IsValid _ownerstaminacomponentt
        (:Is%20Valid
          (bind _bsuccess (Default|TryConsumeStamina _ownerstaminacomponentt _staminacost))
          (if _bsuccess
            _
            (else
              (return false))))
        (:Is%20Not%20Valid
          _))
      (Default|PlayAttack (Variables|Default|GetOwnerCharacter) _attackmontage)
      (Variables|Default|SetCurrentAttackData InAttackData)
      (return true))))

(fn Initialize
  (params (InCharacter :type BP%20Base%20Character%20Object%20Reference) (InStaminaComponent :type BPC%20Stamina%20Object%20Reference))
  (Variables|Default|SetOwnerCharacter InCharacter)
  (Variables|Default|SetOwnerStaminaComponentt InStaminaComponent))

(fn UnequipWeapon)

(fn EndAttack
  (Default|EndTrace (Variables|/Game/MyContents/Weapons/BP_Sword.BP_Sword_C|GetWeaponComponent (Variables|Default|GetCurrentWeapon)))
  (Variables|Default|SetbIsAttacking false))

(fn StartAttack
  (Default|BeginTrace (Variables|/Game/MyContents/Weapons/BP_Sword.BP_Sword_C|GetWeaponComponent (Variables|Default|GetCurrentWeapon)))
  (Variables|Default|SetbIsAttacking true))

(fn PerformAreaAttack
  (params (InAreaAttackData :type ST%20Area%20Attack%20Data%20Structure)))

(fn TryAreaAttack
  (params (InAreaAttackData :type ST%20Area%20Attack%20Data%20Structure)))