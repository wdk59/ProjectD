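; Actor component that manages a stamina pool, starting full and regenerating through timers instead of Tick.
; TryConsumeStamina rejects costs above the current value, otherwise deducts, cancels recharging and sets a delay timer.
; TryConsumeStaminaContinuous only deducts, with StartRechargeDelay available separately to reset that delay.
; StartRecharge runs a looping timer that adds stamina up to the maximum, then clears itself, with debug prints.
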(event Custom|StartRecharge
  (bind _returnvalue (Utilities|Time|SetTimerbyEvent (delegate Custom|RechargeStamina) (Variables|Default|GetRechargeInterval) true))
  (Variables|Default|SetRechargeTimerHandle _returnvalue))

(event Custom|RechargeStamina
  ;[0.15 0.15 0.15 0.5] 스태미너 회복
  (bind _output_get (Variables|Default|SetCurrentStamina (Math|Float|Min(Float) (+ (Variables|Default|GetCurrentStamina) (Variables|Default|GetRechargeAmount)) (Variables|Default|GetMaxStamina))))
  ;[0.15 0.15 0.15 0.5] 스태미너 다 찼으면 회복 타이머 중지
  (if (< _output_get (Variables|Default|GetMaxStamina))
    ;[0 0 1 0.5] Debug
    (Development|PrintString (Class|KismetStringLibrary|BuildStringDouble "" "Recharge Stamina: " _output_get))
    (else
      (Utilities|Time|ClearandInvalidateTimerbyHandle (Variables|Default|GetRechargeTimerHandle))
      (Development|PrintString "Full Stamina"))))

(event Custom|StopRecharge
  (Utilities|Time|ClearandInvalidateTimerbyHandle (Variables|Default|GetRechargeDelayTimerHandle))
  (Utilities|Time|ClearandInvalidateTimerbyHandle (Variables|Default|GetRechargeTimerHandle)))

(event EventBeginPlay
  (Variables|Default|SetCurrentStamina (Variables|Default|GetMaxStamina)))

(event EventTick
  (params (DeltaSeconds :type Float%20%28single-precision%29)))

(fn TryConsumeStamina
  (params (InCost :type Float%20%28double-precision%29))
  (if (> InCost (Variables|Default|GetCurrentStamina))
    (return false)
    (else
      (Variables|Default|SetCurrentStamina (Math|Float|Max(Float) (- (Variables|Default|GetCurrentStamina) InCost) 0.0))
      (CallFunction|StopRecharge)
      (bind _returnvalue (Utilities|Time|SetTimerbyEvent (EventDispatchers|CreateEvent :!event Custom|StartRecharge) (Variables|Default|GetRechargeDelay)))
      (Variables|Default|SetRechargeDelayTimerHandle _returnvalue)
      (return true))))

(fn TryConsumeStaminaContinuous
  (params (InCost :type Float%20%28double-precision%29))
  (if (> InCost (Variables|Default|GetCurrentStamina))
    (return false)
    (else
      (bind _output_get (Variables|Default|SetCurrentStamina (Math|Float|Max(Float) (- (Variables|Default|GetCurrentStamina) InCost) 0.0)))
      (Development|PrintString (Utilities|String|ToString(Float) _output_get))
      (return true))))

(fn StartRechargeDelay
  (CallFunction|StopRecharge)
  (bind _returnvalue (Utilities|Time|SetTimerbyEvent (EventDispatchers|CreateEvent :!event Custom|StartRecharge) (Variables|Default|GetRechargeDelay)))
  (Variables|Default|SetRechargeDelayTimerHandle _returnvalue))