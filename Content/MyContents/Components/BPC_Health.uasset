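; BPC_Health is a health component that tracks its owner's current health.
; It starts at MaxHealth on BeginPlay, clamps Heal to that maximum, and floors ReceiveDamage at zero, calling Die only when damage would push health below zero.
; HealthChanged and Death broadcasts for effects and character death are only PrintString placeholders, and IsDead is never set true.
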(event EventBeginPlay
  (Variables|Default|SetCurrentHealth (Variables|Default|GetMaxHealth))
  (Variables|Default|SetbIsDead false))

(fn Heal
  (params (InHealth :type Float%20%28double-precision%29))
  (Development|PrintString "Boradcast on HealthChanged for 힐 VFX, SFX")
  (if (> (+ (Variables|Default|GetCurrentHealth) InHealth) (Variables|Default|GetMaxHealth))
    (Variables|Default|SetCurrentHealth (Variables|Default|GetMaxHealth))
    (else
      (Variables|Default|SetCurrentHealth (+ (Variables|Default|GetCurrentHealth) InHealth)))))

(fn ReceiveDamage
  (params (InDamage :type Float%20%28double-precision%29))
  (Development|PrintString "Broadcast on HealthChanged for 피격 VFX, SFX")
  (if (< (- (Variables|Default|GetCurrentHealth) InDamage) 0.0)
    (CallFunction|Die)
    (Variables|Default|SetCurrentHealth 0.0)
    (else
      (Variables|Default|SetCurrentHealth (- (Variables|Default|GetCurrentHealth) InDamage)))))

(fn GetHealth
  (return (Variables|Default|GetCurrentHealth)))

(fn Die
  (Development|PrintString "Boradcast on Death for Die Character"))